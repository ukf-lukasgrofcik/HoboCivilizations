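; Barrel tile Blueprint, a child tile that dresses itself with a trashcan prop and two trees and carries a scrap value, name and description.
; BeginPlay runs the parent logic, scatters the props with random offsets and yaw, hides them at zero scale, then sets the tile's data.
; The Grow event reveals the props by instantly setting a random, non-uniform scale on each.
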(event EventBeginPlay
  (bind _trashcansbp (Variables|Default|GetTrashcansBP))
  (bind _treebp1 (Variables|Default|GetTreeBP1))
  (bind _treebp (Variables|Default|GetTreeBP))
  (|CallParentFunction)
  (Transformation|SetRelativeLocationAndRotation _trashcansbp (Math|Vector|MakeVector (Math|Random|RandomFloatinRange -2e+01 6e+01) (Math|Random|RandomFloatinRange 0.0 5e+01) 0.0) (Math|Rotator|MakeRotator 0.0 0.0 (Math|Random|RandomFloatinRange 0.0 3.6e+02)) false false)
  (Transformation|SetRelativeScale3D _trashcansbp "0, 0, 0")
  (Transformation|SetRelativeLocationAndRotation _treebp (Math|Vector|MakeVector (Math|Random|RandomFloatinRange 6e+01 1.2e+02) (Math|Random|RandomFloatinRange -3e+01 1.1e+02) 0.0) (Math|Rotator|MakeRotator 0.0 0.0 (Math|Random|RandomFloatinRange 0.0 3.6e+02)) false false)
  (Transformation|SetRelativeScale3D _treebp "0, 0, 0")
  (Transformation|SetRelativeLocationAndRotation _treebp1 (Math|Vector|MakeVector (Math|Random|RandomFloatinRange -9e+01 9e+01) (Math|Random|RandomFloatinRange -7e+01 -1.3e+02) 0.0) (Math|Rotator|MakeRotator 0.0 0.0 (Math|Random|RandomFloatinRange 0.0 3.6e+02)) false false)
  (Transformation|SetRelativeScale3D _treebp1 "0, 0, 0")
  (Variables|Default|Setscraps 2.0)
  (Variables|Default|Setname (Variables|Default|Getname_0))
  (Variables|Default|Setdescription (Variables|Default|Getdescription_0)))

(event Collision|EventActorBeginOverlap
  (params (OtherActor :type Actor%20Object%20Reference))
  (|CallParentFunction OtherActor) ; This node is disabled and will not be called.\nDrag off pins to build functionality.
)

(event EventTick
  (params (DeltaSeconds :type Float%20%28single-precision%29))
  (|CallParentFunction DeltaSeconds) ; This node is disabled and will not be called.\nDrag off pins to build functionality.
)

(event EventGrow
  (Transformation|SetRelativeScale3D (Variables|Default|GetTrashcansBP) (Math|Vector|MakeVector (Math|Random|RandomFloatinRange 0.2 0.3) (Math|Random|RandomFloatinRange 0.2 0.3) (Math|Random|RandomFloatinRange 0.2 0.3)))
  (Transformation|SetRelativeScale3D (Variables|Default|GetTreeBP) (Math|Vector|MakeVector (Math|Random|RandomFloatinRange 0.2 0.3) (Math|Random|RandomFloatinRange 0.2 0.3) (Math|Random|RandomFloatinRange 0.2 0.3)))
  (Transformation|SetRelativeScale3D (Variables|Default|GetTreeBP1) (Math|Vector|MakeVector (Math|Random|RandomFloatinRange 0.2 0.3) (Math|Random|RandomFloatinRange 0.2 0.3) (Math|Random|RandomFloatinRange 0.2 0.3))))

(fn ConstructionScript
  (|CallParentFunction))