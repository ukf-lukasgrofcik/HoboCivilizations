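; PicnicTileBP is a picnic tile actor that carries a food value, a name and a description.
; On BeginPlay it runs the parent logic, shrinks its table component to zero scale and sets those three values.
; Its Grow event reveals the table by setting it straight to a small uniform scale, with no animation.
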(event EventBeginPlay
  (|CallParentFunction)
  (Transformation|SetRelativeScale3D (Variables|Default|GetTableBP) "0, 0, 0")
  (Variables|Default|Setfood 2.0)
  (Variables|Default|Setname (Variables|Default|Getname_0))
  (Variables|Default|Setdescription (Variables|Default|Getdescription_0)))

(event Collision|EventActorBeginOverlap
  (params (OtherActor :type Actor%20Object%20Reference))
  (|CallParentFunction OtherActor) ; This node is disabled and will not be called.\nDrag off pins to build functionality.
)

(event EventTick
  (params (DeltaSeconds :type Float%20%28single-precision%29))
  (|CallParentFunction DeltaSeconds) ; This node is disabled and will not be called.\nDrag off pins to build functionality.
)

(event EventGrow
  (Transformation|SetRelativeScale3D (Variables|Default|GetTableBP) (Math|Vector|MakeVector 0.2 0.2 0.2)))

(fn ConstructionScript
  (|CallParentFunction))