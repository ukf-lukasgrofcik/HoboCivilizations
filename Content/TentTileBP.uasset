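; TentTileBP is a tile Blueprint that varies the placement of its Tent component.
; On BeginPlay it runs the parent logic, then gives the tent a random relative X/Y offset within fixed bounds and a random yaw.
; The randomization happens at runtime, as the construction script only calls its parent and the Tick and overlap events are disabled stubs.
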(event EventBeginPlay
  (|CallParentFunction)
  (Transformation|SetRelativeLocationAndRotation (Variables|Default|GetTent) (Math|Vector|MakeVector (Math|Random|RandomFloatinRange -3e+01 8e+01) (Math|Random|RandomFloatinRange -5e+01 5e+01) 0.0) (Math|Rotator|MakeRotator 0.0 0.0 (Math|Random|RandomFloatinRange 0.0 3.6e+02)) false false))

(event Collision|EventActorBeginOverlap
  (params (OtherActor :type Actor%20Object%20Reference))
  (|CallParentFunction OtherActor) ; This node is disabled and will not be called.\nDrag off pins to build functionality.
)

(event EventTick
  (params (DeltaSeconds :type Float%20%28single-precision%29))
  (|CallParentFunction DeltaSeconds) ; This node is disabled and will not be called.\nDrag off pins to build functionality.
)

(fn ConstructionScript
  (|CallParentFunction))